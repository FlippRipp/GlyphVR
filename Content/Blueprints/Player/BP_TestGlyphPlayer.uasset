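; Test VR player pawn for drawing glyphs in the air with motion controllers, loading them from file on BeginPlay and saving on EndPlay.
; Main-hand trigger press sets a camera-facing draw plane at the controller.
; While held, Tick feeds controller position to OnControllerDrawingGlyph and moves a Niagara trail to the result; release calls OnGlyphFinished.
; Off-hand trigger saves the current glyph, with handedness resolved through the LeftHandedBranch macro.
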(event EventBeginPlay
  (Class|GlyphPlayer|LoadGlyphsfromFile))

(event Collision|EventActorBeginOverlap
  (params (OtherActor :type Actor%20Object%20Reference)))

(event EventTick
  (params (DeltaSeconds :type Float%20%28single-precision%29))
  (Utilities|FlowControl|Sequence
    (:then_0
      (if (Variables|Default|GetIsTriggerPressed)
        (bind _returnvalue (Class|GlyphPlayer|OnControllerDrawingGlyph (Transformation|GetWorldLocation (CallFunction|GetMainHandController))))
        (Transformation|SetWorldLocation (Variables|Default|GetNiagara) _returnvalue false false)))))

(event EventEndPlay
  (params (EndPlayReason :type EEndPlayReason%20Enum :default "Destroyed"))
  (Class|GlyphPlayer|SaveGlyphstoFile))

(event Input|ActionEvents|InputActionTriggerRight
  (params (Key :type Key%20Structure :default "None"))
  (bind _niagara (Variables|Default|GetNiagara))
  (:Pressed
    (Utilities|LeftHandedBranch
      (:Lefthanded
        (Class|GlyphPlayer|SaveCurrentGlyph)
        (Niagara|ReinitializeSystem (Variables|Default|GetNiagara)))
      (:RightHannded
        (Variables|Default|SetIsTriggerPressed true)
        (Class|GlyphPlayer|SetDrawPlane (Transformation|GetWorldLocation (CallFunction|GetMainHandController)) (Math|Vector|NegateVector (Math|Vector|GetForwardVector (Variables|Default|GetCamera))))
        (Niagara|ReinitializeSystem _niagara)
        (Transformation|SetWorldLocation _niagara (Transformation|GetWorldLocation (CallFunction|GetMainHandController)) false false))))
  (:Released
    (Utilities|LeftHandedBranch
      (:RightHannded
        (Variables|Default|SetIsTriggerPressed false)
        (Class|GlyphPlayer|OnGlyphFinished)))))

(event Input|ActionEvents|InputActionTriggerLeft
  (params (Key :type Key%20Structure :default "None"))
  (bind _niagara (Variables|Default|GetNiagara))
  (:Pressed
    (Utilities|LeftHandedBranch
      (:Lefthanded
        (Variables|Default|SetIsTriggerPressed true)
        (Class|GlyphPlayer|SetDrawPlane (Transformation|GetWorldLocation (CallFunction|GetMainHandController)) (Math|Vector|NegateVector (Math|Vector|GetForwardVector (Variables|Default|GetCamera))))
        (Niagara|ReinitializeSystem _niagara)
        (Transformation|SetWorldLocation _niagara (Transformation|GetWorldLocation (CallFunction|GetMainHandController)) false false))
      (:RightHannded
        (Class|GlyphPlayer|SaveCurrentGlyph)
        (Niagara|ReinitializeSystem (Variables|Default|GetNiagara)))))
  (:Released
    (Utilities|LeftHandedBranch
      (:Lefthanded
        (Variables|Default|SetIsTriggerPressed false)
        (Class|GlyphPlayer|OnGlyphFinished)))))

(fn ConstructionScript)

(fn GetMainHandController
  (Utilities|LeftHandedBranch
    (:Lefthanded
      (return (Variables|Default|GetLeftMotionController)))
    (:RightHannded
      (return (Variables|Default|GetRightMotionController)))))