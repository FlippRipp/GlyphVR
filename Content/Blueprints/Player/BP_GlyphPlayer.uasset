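; BP_GlyphPlayer is a motion-controller player Blueprint for drawing glyphs with the main hand.
; The trigger on the dominant hand sets a pressed flag, with a LeftHandedBranch macro routing input and controller choice by handedness.
; While pressed, Tick feeds that controller's world location to OnControllerDrawingGlyph, then moves a Niagara effect to the returned position and prints it for debugging.
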(event EventBeginPlay)

(event Collision|EventActorBeginOverlap
  (params (OtherActor :type Actor%20Object%20Reference)))

(event EventTick
  (params (DeltaSeconds :type Float%20%28single-precision%29))
  (Utilities|FlowControl|Sequence
    (:then_0
      (if (Variables|Default|GetIsTriggerPressed)
        (bind _returnvalue (Class|GlyphPlayer|OnControllerDrawingGlyph (Transformation|GetWorldLocation (CallFunction|GetMainHandController))))
        (Transformation|SetWorldLocation (Variables|Default|GetNiagara) _returnvalue false false)
        (Development|PrintString (Utilities|String|ToString(Vector) _returnvalue))))))

(event Input|ActionEvents|InputActionTriggerRight
  (params (Key :type Key%20Structure :default "None"))
  (:Pressed
    (Utilities|LeftHandedBranch
      (:RightHannded
        (Variables|Default|SetIsTriggerPressed true))))
  (:Released
    (Utilities|LeftHandedBranch
      (:RightHannded
        (Variables|Default|SetIsTriggerPressed false)))))

(event Input|ActionEvents|InputActionTriggerLeft
  (params (Key :type Key%20Structure :default "None"))
  (:Pressed
    (Utilities|LeftHandedBranch
      (:Lefthanded
        (Variables|Default|SetIsTriggerPressed true))))
  (:Released
    (Utilities|LeftHandedBranch
      (:Lefthanded
        (Variables|Default|SetIsTriggerPressed false)))))

(fn ConstructionScript)

(fn GetMainHandController
  (Utilities|LeftHandedBranch
    (:Lefthanded
      (return (Variables|Default|GetLeftMotionController)))
    (:RightHannded
      (return (Variables|Default|GetRightMotionController)))))