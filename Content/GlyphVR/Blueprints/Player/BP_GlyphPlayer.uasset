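; VR player Blueprint for drawing spell glyphs in the air with motion controllers, supporting either hand as dominant.
; The main trigger sets a camera-facing draw plane and lays Niagara trails along it; the A button finishes the glyph and clears trails.
; Drawn glyphs return by event, are classified by ID as spell circle, element or shape, checked against combination rules, and passed to a spawned VFX controller.
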(event Custom|OnGlyphDrawn_Event
  (params (GlyphDrawn :type Glyph%20Data%20Asset%20Object%20Reference))
  (CallFunction|SpawnGlyph GlyphDrawn)
  (Variables|Default|SetIsPlayerDrawingGlyph false))

(event EventBeginPlay
  (EventDispatchers|AssignOnGlyphDrawn (delegate Custom|OnGlyphDrawn_Event))
  (bind _returnvalue (Game|SpawnActorfromClass "/Game/GlyphVR/Blueprints/Glyphs/BP_GLyphVFXController.BP_GLyphVFXController_C" (Math|Conversions|ToTransform(Vector) (Transformation|GetWorldLocation (Variables|Default|GetCamera))) "Undefined" 0 0))
  (bind _output_get (Variables|Default|SetGlyphVFXController _returnvalue))
  (Variables|/Game/GlyphVR/Blueprints/Glyphs/BP_GLyphVFXController.BP_GLyphVFXController_C|SetPlayer _output_get (Variables|Default|GetCamera)))

(event EventTick
  (params (DeltaSeconds :type Float%20%28single-precision%29))
  (CallFunction|TriggerHeldCheck)
  (Effects|Components|ParticleSystem|SetVectorParameter (Variables|Default|GetNiagara1) "BeamEnd" (Transformation|GetWorldLocation (Variables|Default|GetRightMotionController))))

(event EventEndPlay
  (params (EndPlayReason :type EEndPlayReason%20Enum :default "Destroyed")))

(event Input|ActionEvents|InputActionTriggerRight
  (params (Key :type Key%20Structure))
  (:Pressed
    (Utilities|MainHanndBranch
      (:Lefthanded
        (CallFunction|OffTriggerDown)
        (Variables|Default|SetIsOffTriggerHeld true))
      (:RightHannded
        (CallFunction|MainTriggerDown)
        (Variables|Default|SetIsMainTriggerHeld true))))
  (:Released
    (Utilities|MainHanndBranch
      (:Lefthanded
        (CallFunction|OffTriggerUp)
        (Variables|Default|SetIsOffTriggerHeld false))
      (:RightHannded
        (CallFunction|MainTriggerUp)
        (Variables|Default|SetIsMainTriggerHeld false)))))

(event Input|ActionEvents|InputActionTriggerLeft
  (params (Key :type Key%20Structure))
  (:Pressed
    (Utilities|MainHanndBranch
      (:Lefthanded
        (CallFunction|MainTriggerDown)
        (Variables|Default|SetIsMainTriggerHeld true))
      (:RightHannded
        (CallFunction|OffTriggerDown)
        (Variables|Default|SetIsOffTriggerHeld true))))
  (:Released
    (Utilities|MainHanndBranch
      (:Lefthanded
        (CallFunction|MainTriggerUp)
        (Variables|Default|SetIsMainTriggerHeld false))
      (:RightHannded
        (CallFunction|OffTriggerUp)
        (Variables|Default|SetIsOffTriggerHeld false)))))

(event Input|ActionEvents|InputActionRIghtAButton
  (params (Key :type Key%20Structure))
  (:Pressed
    (Utilities|MainHanndBranch
      (:RightHannded
        (if (Variables|Default|GetIsPlayerDrawingGlyph)
          (Class|GlyphPlayer|OnGlyphFinished)
          (CallFunction|DeleteNiagaraTrails))))))

(event Input|ActionEvents|InputActionLeftAButton
  (params (Key :type Key%20Structure))
  (:Pressed
    (Utilities|MainHanndBranch
      (:Lefthanded
        (if (Variables|Default|GetIsPlayerDrawingGlyph)
          (Class|GlyphPlayer|OnGlyphFinished)
          (CallFunction|DeleteNiagaraTrails))))))

(fn ConstructionScript)

(fn GetMainHandController
  (Utilities|MainHanndBranch
    (:Lefthanded
      (return (Variables|Default|GetLeftMotionController)))
    (:RightHannded
      (return (Variables|Default|GetRightMotionController)))))

(fn MainTriggerDown
  (bind _camera (Variables|Default|GetCamera))
  (bind _returnvalue (Math|Vector|GetForwardVector _camera))
  (bind _returnvalue_2 (Math|Vector|NegateVector _returnvalue))
  (if (Variables|Default|GetIsPlayerDrawingGlyph)
    _
    (else
      (Class|GlyphPlayer|SetDrawPlane (Transformation|GetWorldLocation (CallFunction|GetMainHandController)) (Math|Vector|MakeVector (.x _returnvalue_2) (.y _returnvalue_2) 0.0))))
  (CallFunction|StartNiagaraTrail)
  (Variables|Default|SetIsPlayerDrawingGlyph true))

(fn MainTriggerUp)

(fn MainTriggerHeld
  (bind _returnvalue (Class|GlyphPlayer|OnControllerDrawingGlyph (Transformation|GetWorldLocation (CallFunction|GetMainHandController))))
  (Transformation|SetWorldLocation (Variables|Default|GetCurrentNiagaraTrail) _returnvalue false false))

(fn OffTriggerDown)

(fn OffTriggerUp)

(fn OffTriggerHeld)

(fn TriggerHeldCheck
  (Utilities|FlowControl|Sequence
    (:then_0
      (if (Variables|Default|GetIsMainTriggerHeld)
        (CallFunction|MainTriggerHeld)))
    (:then_1
      (if (Variables|Default|GetIsOffTriggerHeld)
        (CallFunction|OffTriggerHeld)))))

(fn SpawnGlyph
  (params (Glyph :type Glyph%20Data%20Asset%20Object%20Reference))
  (bind _output_get (LocalVariables|SetInputGlyph Glyph))
  (Utilities|GetGlyphType _output_get
    (:SpellCircle
      (Utilities|CanAddSpellCircle
        (:Succsess
          (Variables|Default|SetHasSpellCircle true))
        (:Failed
          (Default|SpellFailed (Variables|Default|GetGlyphVFXController))))
      (Default|AddSpellCircle (Variables|Default|GetGlyphVFXController) (LocalVariables|GetInputGlyph)))
    (:Element
      (Utilities|CanAddElementGlyph
        (:Succsess
          (Utilities|Array|Add (Variables|Default|GetElementGlyphsIds) (Variables|/Script/GlyphVR.GlyphDataAsset|GetGlyphID (LocalVariables|GetInputGlyph))))
        (:Failed
          (Default|SpellFailed (Variables|Default|GetGlyphVFXController))))
      (Default|AddElementGlyph (Variables|Default|GetGlyphVFXController) (LocalVariables|GetInputGlyph)))
    (:Shape
      (Utilities|CanAddShapeGlyph
        (:Succsess
          (Utilities|Array|Add (Variables|Default|GetShapeGlyphsIds) (Variables|/Script/GlyphVR.GlyphDataAsset|GetGlyphID (LocalVariables|GetInputGlyph))))
        (:Failed
          (Default|SpellFailed (Variables|Default|GetGlyphVFXController))))
      (Default|AddShapeGlyph (Variables|Default|GetGlyphVFXController) (LocalVariables|GetInputGlyph))))
  (return))

(fn StartNiagaraTrail
  (bind _returnvalue (Game|AddComponentbyClass "/Script/Niagara.NiagaraComponent" false))
  (Class|NiagaraComponent|SetAsset _returnvalue "/Game/GlyphVR/Blueprints/Player/GlyphLine.GlyphLine" true)
  (bind _output_get (Variables|Default|SetCurrentNiagaraTrail _returnvalue))
  (Utilities|Array|Add (Variables|Default|GetNiagaraTrails) _output_get))

(fn DeleteNiagaraTrails
  (bind _niagaratrails (Variables|Default|GetNiagaraTrails))
  (for _index (range 0 (- (Utilities|Array|Length (Variables|Default|GetNiagaraTrails)) 1))
    (Components|DestroyComponent (Utilities|Array|Get(acopy) _niagaratrails _index)))
  (Utilities|Array|Clear _niagaratrails)
  (Variables|Default|SetCurrentNiagaraTrail 0))

(fn ClearActiveGlyphs
  (Default|ClearGlyphs (Variables|Default|GetGlyphVFXController))
  (Utilities|Array|Clear (Variables|Default|GetShapeGlyphsIds))
  (Utilities|Array|Clear (Variables|Default|GetElementGlyphsIds)))