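; Glyph VFX controller that displays the spell circle, element glyphs and shape glyphs of a spell in front of the player.
; Add functions spawn each glyph's actor, and Tick keeps the controller ahead of the Player component, facing it.
; Element glyphs orbit the center on a sine/cosine ring while shape glyphs line up in a row.
; Finishing clears all glyphs immediately; failing clears them after a short delay.
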(event EventBeginPlay)

(event Collision|EventActorBeginOverlap
  (params (OtherActor :type Actor%20Object%20Reference)))

(event EventTick
  (params (DeltaSeconds :type Float%20%28single-precision%29))
  (CallFunction|GlyphAnimation DeltaSeconds)
  (if (Variables|Default|GetIsSpellFailing)
    (Utilities|DelayedClear)))

(fn ConstructionScript)

(fn SpellFailed
  (Variables|Default|SetIsSpellFailing true))

(fn AddElementGlyph
  (params (Glyph :type Glyph%20Data%20Asset%20Object%20Reference))
  (bind _returnvalue (Game|SpawnActorfromClass (Variables|/Script/GlyphVR.GlyphDataAsset|GetGlyphActor Glyph) (Math|Conversions|ToTransform(Vector) (Transformation|GetActorLocation)) "Undefined" 0 0))
  (Utilities|Array|Add (Variables|Default|GetElementGlyphs) _returnvalue))

(fn AddShapeGlyph
  (params (Glyph :type Glyph%20Data%20Asset%20Object%20Reference))
  (bind _returnvalue (Game|SpawnActorfromClass (Variables|/Script/GlyphVR.GlyphDataAsset|GetGlyphActor Glyph) (Math|Conversions|ToTransform(Vector) (Transformation|GetActorLocation)) "Undefined" 0 0))
  (Utilities|Array|Add (Variables|Default|GetShapeGlyphs) _returnvalue)
  (for (_array_element _array_index) (Variables|Default|GetShapeGlyphs)
    (Transformation|SetActorRelativeLocation _array_element (Math|Vector|MakeVector 0.0 (+ (/ (- 0.0 (* (Utilities|Array|Length (Variables|Default|GetShapeGlyphs)) (Variables|Default|GetShapeRuneSpace))) 1.0) (* _array_index (Variables|Default|GetShapeRuneSpace))) 0.0))))

(fn AddSpellCircle
  (params (Glyph :type Glyph%20Data%20Asset%20Object%20Reference))
  (bind _returnvalue (Game|SpawnActorfromClass (Variables|/Script/GlyphVR.GlyphDataAsset|GetGlyphActor Glyph) (Math|Conversions|ToTransform(Vector) (Transformation|GetActorLocation)) "Undefined" 0 0))
  (Variables|Default|SetSpellCircle _returnvalue))

(fn ClearGlyphs
  (bind _spellcircle (Variables|Default|GetSpellCircle))
  (Utilities|IsValid _spellcircle
    (:Is%20Valid
      (Actor|SetLifeSpan _spellcircle 0.001))
    (:Is%20Not%20Valid
      _))
  (CallFunction|ClearElementGlyphs)
  (CallFunction|ClearShapeGlyphs)
  (Variables|Default|SetHasSpellCircle false))

(fn ClearElementGlyphs
  (bind _elementglyphs (Variables|Default|GetElementGlyphs))
  (bind _output (Utilities|Array|Get(acopy) _elementglyphs))
  (while (!= (Utilities|Array|Length _elementglyphs) 0)
    (Actor|SetLifeSpan _output 0.05)
    (Utilities|Array|RemoveItem _elementglyphs _output))
  (Utilities|Array|Clear _elementglyphs))

(fn ClearShapeGlyphs
  (bind _shapeglyphs (Variables|Default|GetShapeGlyphs))
  (bind _output (Utilities|Array|Get(acopy) _shapeglyphs))
  (while (!= (Utilities|Array|Length _shapeglyphs) 0)
    (Actor|SetLifeSpan _output 0.05)
    (Utilities|Array|RemoveItem _shapeglyphs _output))
  (Utilities|Array|Clear _shapeglyphs))

(fn GlyphAnimation
  (params (DeltaTime :type Float%20%28single-precision%29))
  (bind _player (Variables|Default|GetPlayer))
  (bind _spellcircle (Variables|Default|GetSpellCircle))
  (bind _player_2 (Variables|Default|GetPlayer))
  ;[1 0.9703 0] Spell Circle Position and rotation
  (Utilities|IsValid _spellcircle
    (:Is%20Valid
      (Transformation|SetActorRotation _spellcircle (Transformation|GetActorRotation))
      (Transformation|SetActorLocation _spellcircle (Transformation|GetActorLocation) false false))
    (:Is%20Not%20Valid
      _))
  (Utilities|FlowControl|Sequence
    (:then_0
      ;[1 0.3466 0.08404] Element Glyphs Rotation
      (Variables|Default|SetRotationOffset (+ DeltaTime (Variables|Default|GetRotationOffset)))
      (for (_array_element _array_index) (Variables|Default|GetElementGlyphs)
        (Transformation|SetActorLocation _array_element (+ (* (Transformation|GetActorRightVector) (* (Math|Trig|Cos(Radians) (+ (Variables|Default|GetRotationOffset) (* _array_index (/ (* (Math|Trig|GetPI) 2.0) (Math|Conversions|ToFloat(Integer) (Utilities|Array|Length (Variables|Default|GetElementGlyphs))))))) (Variables|Default|GetSpellCircleRadius))) (* (Transformation|GetActorUpVector) (* (Math|Trig|Sin(Radians) (+ (Variables|Default|GetRotationOffset) (* _array_index (/ (* (Math|Trig|GetPI) 2.0) (Math|Conversions|ToFloat(Integer) (Utilities|Array|Length (Variables|Default|GetElementGlyphs))))))) (Variables|Default|GetSpellCircleRadius))) (Transformation|GetActorLocation)) false false)
        (Transformation|SetActorRotation _array_element (Transformation|GetActorRotation)))
      ;[0.1604 1 0.2645] VFX Position and rotation
      (Utilities|IsValid _player
        (:Is%20Valid
          (Transformation|SetActorRotation (Math|Rotator|FindLookatRotation (Transformation|GetActorLocation) (Transformation|GetWorldLocation _player)))
          (Transformation|SetActorLocation (+ (Transformation|GetWorldLocation _player_2) (* (Math|Vector|GetForwardVector _player_2) 1e+02)) false false))))
    (:then_1
      ;[0 0.3082 1] Shape Glyphs Positions and rotation
      (for (_array_element_2 _array_index_2) (Variables|Default|GetShapeGlyphs)
        (Transformation|SetActorLocation _array_element_2 (+ (* (Transformation|GetActorRightVector) (+ (/ (- 0.0 (* (Utilities|Array|Length (Variables|Default|GetShapeGlyphs)) (Variables|Default|GetShapeRuneSpace))) 2.0) (* _array_index_2 (Variables|Default|GetShapeRuneSpace)))) (Transformation|GetActorLocation)) false false)
        (Transformation|SetActorRotation _array_element_2 (Transformation|GetActorRotation))))))

(fn FinishSpell
  (CallFunction|ClearGlyphs))