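; BP_Dummy is an enemy dummy that reacts to damage events and displays burning and doused status.
; On BeginPlay it binds to its Damage component's damage, doused and burning delegates.
; The status changes toggle the visibility of the Doused and Burning components.
; Each damage type in a hit is passed with the impact point to ApplyEffect, whose switch on type has no visible handling.
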(event Custom|OnIsDousedChanged_Event
  (params (State :type Boolean))
  (Rendering|SetVisibility (Variables|Default|GetDoused) State false))

(event Custom|OnDamage_Event_0
  (params (Damage :type Float%20%28single-precision%29) (DamageTypes :type Array%20of%20GlyphEnum%20Enums :default "SpellCircle") (ImpactPoint :type Vector))
  (for _array_element DamageTypes
    (CallFunction|ApplyEffect _array_element ImpactPoint)))

(event Custom|OnIsBurningChanged_Event
  (params (State :type Boolean))
  (Rendering|SetVisibility (Variables|Default|GetBurning) State false))

(event EventBeginPlay
  (EventDispatchers|AssignOnDamage (Variables|Default|GetDamage) (delegate Custom|OnDamage_Event_0))
  (EventDispatchers|AssignOnIsDousedChanged (Variables|Default|GetDamage) (delegate Custom|OnIsDousedChanged_Event))
  (EventDispatchers|AssignOnIsBurningChanged (Variables|Default|GetDamage) (delegate Custom|OnIsBurningChanged_Event)))

(event Collision|EventActorBeginOverlap
  (params (OtherActor :type Actor%20Object%20Reference)))

(event EventTick
  (params (DeltaSeconds :type Float%20%28single-precision%29)))

(fn ConstructionScript)

(fn ApplyEffect
  (params (Type :type GlyphEnum%20Enum :default "SpellCircle") (ImpactPoint :type Vector))
  (switch Utilities|FlowControl|Switch|SwitchonGlyphEnum Type))