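; BP_ProjectileSpell is a projectile spell actor in GlyphVR that displays visuals for the elements it is created with.
; On BeginPlay it binds to an OnInit event and hides its Fire, Earth and Water components.
; When OnInit fires, InitProjectile loops through the passed elements and makes each matching component visible.
; The file contains no movement or hit logic, as Tick and overlap events are empty.
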(event Custom|OnInit_Event_0
  (params (Elements :type Array%20of%20GlyphEnum%20Enums :default "SpellCircle"))
  (CallFunction|InitProjectile Elements))

(event EventBeginPlay
  (EventDispatchers|AssignOnInit (delegate Custom|OnInit_Event_0))
  (Rendering|SetVisibility (Variables|Default|GetFire) false false)
  (Rendering|SetVisibility (Variables|Default|GetEarth) false false)
  (Rendering|SetVisibility (Variables|Default|GetWater) false false))

(event Collision|EventActorBeginOverlap
  (params (OtherActor :type Actor%20Object%20Reference)))

(event EventTick
  (params (DeltaSeconds :type Float%20%28single-precision%29)))

(fn ConstructionScript)

(fn InitProjectile
  (params (elements :type Array%20of%20GlyphEnum%20Enums :default "SpellCircle"))
  (for _array_element elements
    (switch Utilities|FlowControl|Switch|SwitchonGlyphEnum _array_element
      (:Fire
        (Rendering|SetVisibility (Variables|Default|GetFire) true false))
      (:Earth
        (Rendering|SetVisibility (Variables|Default|GetEarth) true false))
      (:Water
        (Rendering|SetVisibility (Variables|Default|GetWater) true false)))))