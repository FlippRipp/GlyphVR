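; BP_beamSpell is the visual for a beam spell that stretches from its source to an impact point.
; On init it stores the source and shows the Fire, Water or Earth layers matching the spell's elements.
; On impact it centers, orients and length-scales the beam between both points, scaling the dynamic materials' Y tiling with distance.
; Air and fire-smoke Niagara spawns are present but unconnected.
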(event Custom|OnImpact_Event
  (params (ImpactPoint :type Vector) (ImpactDirection :type Vector) (Elements :type Array%20of%20GlyphEnum%20Enums :default "SpellCircle") (VFX :type Array%20of%20Spell%20Effect%20Class%20References) (Target :type Actor%20Object%20Reference))
  (bind _source (Variables|Default|GetSource))
  (bind _returnvalue (Transformation|GetWorldLocation _source))
  (bind _returnvalue_2 (Math|Vector|Distance(Vector) ImpactPoint _returnvalue))
  (bind _returnvalue_3 (/ _returnvalue_2 1e+02))
  (Transformation|SetRelativeScale3D (Variables|Default|GetBeam) (Math|Vector|MakeVector 0.2 0.2 _returnvalue_3))
  (Rendering|Material|SetScalarParameterValue (Variables|Default|GetFireDynamicMaterial) "Tiling Y" _returnvalue_3 :!class /Script/Engine.MaterialInstanceDynamic)
  (Rendering|Material|SetScalarParameterValue (Variables|Default|GetWaterDynamicMaterial) "Tiling Y" _returnvalue_3 :!class /Script/Engine.MaterialInstanceDynamic)
  (Rendering|Material|SetScalarParameterValue (Variables|Default|GetEarthDynamicMaterial) "Tiling Y" _returnvalue_3 :!class /Script/Engine.MaterialInstanceDynamic)
  (Transformation|SetWorldRotation (Variables|Default|GetBeam) (Math|Rotator|FindLookatRotation ImpactPoint _returnvalue) false false)
  (Transformation|SetWorldLocation (Variables|Default|GetBeam) (Math|Vector|Lerp(Vector) ImpactPoint _returnvalue 0.5) false false))

(event Custom|OnInit_Event
  (params (Elements :type Array%20of%20GlyphEnum%20Enums :default "SpellCircle") (Source :type Scene%20Component%20Object%20Reference))
  (Components|InitBeam Elements)
  (Variables|Default|SetSource Source))

(event EventBeginPlay
  (EventDispatchers|AssignOnImpact (delegate Custom|OnImpact_Event))
  (EventDispatchers|AssignOnInit (delegate Custom|OnInit_Event))
  (Rendering|SetVisibility (Variables|Default|GetFire) false false)
  (Rendering|SetVisibility (Variables|Default|GetWater) false false)
  (Rendering|SetVisibility (Variables|Default|GetEarth) false false))

(fn ConstructionScript
  (bind _returnvalue (Rendering|Material|CreateDynamicMaterialInstance (Variables|Default|GetFire) 0 "/Game/GlyphVR/Materials/m_ProjectileFire.m_ProjectileFire" "None" :!class /Script/Engine.PrimitiveComponent))
  (Variables|Default|SetFireDynamicMaterial _returnvalue)
  (bind _returnvalue_2 (Rendering|Material|CreateDynamicMaterialInstance (Variables|Default|GetWater) 0 "/Game/GlyphVR/Materials/m_ProjectileWater.m_ProjectileWater" "None" :!class /Script/Engine.PrimitiveComponent))
  (Variables|Default|SetWaterDynamicMaterial _returnvalue_2)
  (bind _returnvalue_3 (Rendering|Material|CreateDynamicMaterialInstance (Variables|Default|GetEarth) 0 "/Game/GlyphVR/Materials/m_ProjectileEarth.m_ProjectileEarth" "None" :!class /Script/Engine.PrimitiveComponent))
  (bind _output_get (Variables|Default|SetEarthDynamicMaterial _returnvalue_3))
  (Rendering|Material|SetScalarParameterValue _output_get "PanningX" 0.3 :!class /Script/Engine.MaterialInstanceDynamic)
  (Rendering|Material|SetScalarParameterValue _output_get "PanningY" 0.3 :!class /Script/Engine.MaterialInstanceDynamic))

(fn InitBeam
  (params (elements :type Array%20of%20GlyphEnum%20Enums :default "SpellCircle"))
  (for _array_element elements
    (switch Utilities|FlowControl|Switch|SwitchonGlyphEnum _array_element
      (:Fire
        (Rendering|SetVisibility (Variables|Default|GetFire) true false))
      (:Earth
        (Rendering|SetVisibility (Variables|Default|GetEarth) true false))
      (:Water
        (Rendering|SetVisibility (Variables|Default|GetWater) true false)))))