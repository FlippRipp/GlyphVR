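; BP_ProjectileSpell is a projectile spell actor whose visuals reflect the elements it is made of.
; InitProjectile reveals the Fire, Earth and Water components per element and attaches Niagara effects for Air and Fire smoke.
; BeginPlay hides those three components, binds InitProjectile to OnInit, then also runs it with a debug list of all four elements.
; Overlap and Tick are empty, and the InitSpell call is unconnected.
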(event Custom|OnInit_Event_0
  (params (Elements :type Array%20of%20GlyphEnum%20Enums :default "SpellCircle"))
  (CallFunction|InitProjectile Elements))

(event EventBeginPlay
  (bind _debuginput (Variables|Default|GetDebugInput))
  (EventDispatchers|AssignOnInit (delegate Custom|OnInit_Event_0))
  (Rendering|SetVisibility (Variables|Default|GetFire) false false)
  (Rendering|SetVisibility (Variables|Default|GetEarth) false false)
  (Rendering|SetVisibility (Variables|Default|GetWater) false false)
  (Utilities|Array|Add _debuginput "Air")
  (Utilities|Array|Add _debuginput "Earth")
  (Utilities|Array|Add _debuginput "Fire")
  (Utilities|Array|Add _debuginput "Water")
  (CallFunction|InitProjectile _debuginput))

(event Collision|EventActorBeginOverlap
  (params (OtherActor :type Actor%20Object%20Reference)))

(event EventTick
  (params (DeltaSeconds :type Float%20%28single-precision%29)))

(fn ConstructionScript)

(fn InitProjectile
  (params (elements :type Array%20of%20GlyphEnum%20Enums :default "SpellCircle"))
  (bind _fire (Variables|Default|GetFire))
  (for _array_element elements
    (switch Utilities|FlowControl|Switch|SwitchonGlyphEnum _array_element
      (:Air
        (Niagara|SpawnSystemAttached "/Game/GlyphVR/Niagara/N_Air.N_Air" (Variables|Default|GetAir) "None" "0, 0, 0" "0, 0, 0" "KeepRelativeOffset" false))
      (:Fire
        (Rendering|SetVisibility _fire true false)
        (Niagara|SpawnSystemAttached "/Game/GlyphVR/Niagara/N_FireSmoke.N_FireSmoke" _fire "None" "0, 0, 0" "0, 0, 0" "KeepRelativeOffset" false))
      (:Earth
        (Rendering|SetVisibility (Variables|Default|GetEarth) true false))
      (:Water
        (Rendering|SetVisibility (Variables|Default|GetWater) true false)))))